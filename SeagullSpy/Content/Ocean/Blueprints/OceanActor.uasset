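; Ocean surface actor that follows the first player's pawn horizontally at Z zero, creating an ocean that moves with the player.
; Construction creates a dynamic material on the surface mesh and pushes wave wavelength, amplitude, size and a direction taken from the actor's forward vector.
; Each tick it recenters and feeds the center to the material.
; Wave settings are mirrored to an OceanManager, keeping both in sync.
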(event `self.ReceiveTick`
  (params (DeltaSeconds :type "Float (single-precision)"))
  (bind _returnvalue (`GameplayStatics.GetPlayerPawn` 0))
  (`/Engine/EditorBlueprintResources/StandardMacros.IsValid` _returnvalue
    (:`Is Valid`
      (`self.UpdateCenter` (`KismetMathLibrary.Conv_VectorToVector2D` (`self.K2_GetActorLocation` _returnvalue))))))

(fn `UpdateCenter`
  (params (Center :type "Object.Vector2D Structure"))
  (bind (_x _y) (`KismetMathLibrary.BreakVector2D` Center))
  (bind _dynamicoceanmaterial (`self.DynamicOceanMaterial`))
  (bind _returnvalue (`KismetMathLibrary.MakeVector` _x _y))
  (`self.K2_SetActorLocation` _returnvalue)
  (set `self.Center` _returnvalue)
  (`MaterialInstanceDynamic.SetVectorParameterValue` _dynamicoceanmaterial "Center" (`KismetMathLibrary.Conv_VectorToLinearColor` _returnvalue))
  (`MaterialInstanceDynamic.SetScalarParameterValue` _dynamicoceanmaterial "Size" (`self.Size`)))

(fn `UpdateWaveParameters`
  (params (Wavelength :type "Float (double-precision)") (Amplitude :type "Float (double-precision)") (Direction :type "Object.Vector2D Structure") (Size :type "Float (double-precision)"))
  (bind (_x _y) (`KismetMathLibrary.BreakVector2D` Direction))
  (bind _dynamicoceanmaterial (`self.DynamicOceanMaterial`))
  (bind _oceanmanager (`self.OceanManager`))
  (`|ExecutionSequence`
    (:`then_0`
      (set `self.Wavelength` Wavelength)
      (set `self.Amplitude` Amplitude)
      (set `self.Size` Size))
    (:`then_1`
      ;[1 1 1] Update Material
      (`MaterialInstanceDynamic.SetVectorParameterValue` _dynamicoceanmaterial "Direction" (make `Object.LinearColor` _x _y))
      (`MaterialInstanceDynamic.SetScalarParameterValue` _dynamicoceanmaterial "Wavelength" Wavelength)
      (`MaterialInstanceDynamic.SetScalarParameterValue` _dynamicoceanmaterial "Amplitude" Amplitude)
      (`MaterialInstanceDynamic.SetScalarParameterValue` _dynamicoceanmaterial "Size" (`self.Size`)))
    (:`then_2`
      ;[1 1 1] Update Ocean Manager
      (set `/Game/Ocean/Blueprints/OceanManager.Wavelength` Wavelength _oceanmanager)
      (set `/Game/Ocean/Blueprints/OceanManager.Amplitude` Amplitude _oceanmanager)
      (set `/Game/Ocean/Blueprints/OceanManager.Direction` Direction _oceanmanager))))

(fn `UserConstructionScript`
  (`|ExecutionSequence`
    (:`then_0`
      (bind _returnvalue (`PrimitiveComponent.CreateDynamicMaterialInstance` (`self.OceanSurfaceMesh`) 0 (`self.OceanMaterial`)))
      (`/Engine/EditorBlueprintResources/StandardMacros.IsValid` _returnvalue
        (:`Is Valid`
          (set `self.DynamicOceanMaterial` _returnvalue))))
    (:`then_1`
      (`self.UpdateWaveParameters` (`self.Wavelength`) (`self.Amplitude`) (`KismetMathLibrary.Conv_VectorToVector2D` (`self.GetActorForwardVector`)) (`self.Size`)))))